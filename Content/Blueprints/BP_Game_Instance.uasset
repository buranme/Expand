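; Game instance that persists a procedural planet's data in a single "Background" save slot.
; On Init it loads the existing BP_SaveGame or creates a new one, caching it as SaveGameData.
; Save and load functions copy mesh, shape settings, seeds and material instance between Planet and that object, while a clear function deletes the slot.
; LoadPlanetData reads the cached object; its trailing slot load result is unused.
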(event EventInit
  (bind _background (Variables|Default|GetBackground))
  (bind _returnvalue (SaveGame|DoesSaveGameExist _background))
  (if _returnvalue
    (bind _returnvalue_2 (SaveGame|LoadGamefromSlot _background))
    (bind _asbp_save_game (Utilities|Casting|CastToBP_SaveGame _returnvalue_2))
    (Variables|Default|SetSaveGameData _asbp_save_game)
    (else
      (bind _returnvalue_3 (SaveGame|CreateSaveGameObject "/Game/Blueprints/BP_SaveGame.BP_SaveGame_C"))
      (Variables|Default|SetSaveGameData _returnvalue_3))))

(fn SavePlanetData
  (bind _planet (Variables|Default|GetPlanet))
  (bind _savegamedata (Variables|Default|GetSaveGameData))
  (Variables|/Game/Blueprints/BP_SaveGame.BP_SaveGame_C|SetVertices _savegamedata (Variables|/Script/Expand.SphericalMesh|GetFaceVertices _planet))
  (Variables|/Game/Blueprints/BP_SaveGame.BP_SaveGame_C|SetTriangles _savegamedata (Variables|/Script/Expand.SphericalMesh|GetFaceTriangles _planet))
  (Variables|/Game/Blueprints/BP_SaveGame.BP_SaveGame_C|SetDetail _savegamedata (Variables|/Script/Expand.SphericalMesh|GetDetail _planet))
  (Variables|/Game/Blueprints/BP_SaveGame.BP_SaveGame_C|SetRadius _savegamedata (Variables|/Script/Expand.SphericalMesh|GetRadius _planet))
  (Variables|/Game/Blueprints/BP_SaveGame.BP_SaveGame_C|SetSeeds _savegamedata (Variables|/Script/Expand.SphericalMesh|GetSeeds _planet))
  (Variables|/Game/Blueprints/BP_SaveGame.BP_SaveGame_C|SetMountainRangeSeed _savegamedata (Variables|/Script/Expand.SphericalMesh|GetMountainRangeSeed _planet))
  (Variables|/Game/Blueprints/BP_SaveGame.BP_SaveGame_C|SetMountainRangeMaskSeed _savegamedata (Variables|/Script/Expand.SphericalMesh|GetMountainRangeMaskSeed _planet))
  (Variables|/Game/Blueprints/BP_SaveGame.BP_SaveGame_C|SetMaterialInstance _savegamedata (Variables|/Game/Blueprints/BP_SphericalMesh.BP_SphericalMesh_C|GetCreatedMI _planet))
  (SaveGame|SaveGametoSlot (Variables|Default|GetSaveGameData) (Variables|Default|GetBackground)))

(fn LoadPlanetData
  (bind _planet (Variables|Default|GetPlanet))
  (bind _savegamedata (Variables|Default|GetSaveGameData))
  (Variables|/Script/Expand.SphericalMesh|SetFaceVertices _planet (Variables|/Game/Blueprints/BP_SaveGame.BP_SaveGame_C|GetVertices _savegamedata))
  (Variables|/Script/Expand.SphericalMesh|SetFaceTriangles _planet (Variables|/Game/Blueprints/BP_SaveGame.BP_SaveGame_C|GetTriangles _savegamedata))
  (Variables|/Script/Expand.SphericalMesh|SetDetail _planet (Variables|/Game/Blueprints/BP_SaveGame.BP_SaveGame_C|GetDetail _savegamedata))
  (Variables|/Script/Expand.SphericalMesh|SetRadius _planet (Variables|/Game/Blueprints/BP_SaveGame.BP_SaveGame_C|GetRadius _savegamedata))
  (Variables|/Script/Expand.SphericalMesh|SetSeeds _planet (Variables|/Game/Blueprints/BP_SaveGame.BP_SaveGame_C|GetSeeds _savegamedata))
  (Variables|/Script/Expand.SphericalMesh|SetMountainRangeSeed _planet (Variables|/Game/Blueprints/BP_SaveGame.BP_SaveGame_C|GetMountainRangeSeed _savegamedata))
  (Variables|/Script/Expand.SphericalMesh|SetMountainRangeMaskSeed _planet (Variables|/Game/Blueprints/BP_SaveGame.BP_SaveGame_C|GetMountainRangeMaskSeed _savegamedata))
  (Variables|/Game/Blueprints/BP_SphericalMesh.BP_SphericalMesh_C|SetCreatedMI _planet (Variables|/Game/Blueprints/BP_SaveGame.BP_SaveGame_C|GetMaterialInstance _savegamedata))
  (SaveGame|LoadGamefromSlot (Variables|Default|GetBackground)))

(fn ClearPlanetData
  (SaveGame|DeleteGameinSlot (Variables|Default|GetBackground)))