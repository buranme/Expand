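; BP_ProcMesh is a procedural map experiment built around CityGrowth, which spreads a city across tiles.
; CityGrowth seeds a random tile, then recurses every half second, meshing a random frontier tile and adding its unclaimed candidates from GetTilesFromTile to PotentialCity.
; BeginPlay and construction are empty.
; Setup with mesh and ocean spawning, render-target drawing, river tracing and the initial CityGrowth call are all disconnected.
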(event Custom|CityGrowth
  (bind _potentialcity (Variables|Default|GetPotentialCity))
  (bind _potentialcity_2 (Variables|Default|GetPotentialCity))
  (bind _city (Variables|Default|GetCity))
  (bind _city_2 (Variables|Default|GetCity))
  (Math|Integer|CompareInt 0 (Utilities|Array|Length _city_2)
    (:==
      (bind _returnvalue (Utilities|Array|Add _city_2 (Math|Random|RandomInteger (* 216 216))))
      (Class|ProcMesh|CreateMeshonTile (Utilities|Array|Get(acopy) _city_2 _returnvalue))
      (bind _returnvalue_2 (Class|ProcMesh|GetTilesfromTile (Utilities|Array|Get(acopy) _city_2 _returnvalue)))
      (for _array_element _returnvalue_2
        (Utilities|Array|Add (Variables|Default|GetPotentialCity) _array_element))
      (Utilities|FlowControl|Delay 0.5)
      (CallFunction|CityGrowth))
    (:<
      (bind _returnvalue_3 (Utilities|Array|Add _city (.OutItem (Utilities|Array|Random _potentialcity))))
      (Development|PrintString (Utilities|String|ToString(Integer) (Utilities|Array|Get(acopy) _city _returnvalue_3)))
      (Class|ProcMesh|CreateMeshonTile (Utilities|Array|Get(acopy) _city _returnvalue_3))
      (Utilities|Array|RemoveItem _potentialcity (Utilities|Array|Get(acopy) _city _returnvalue_3))
      (bind _returnvalue_4 (Class|ProcMesh|GetTilesfromTile (Utilities|Array|Get(acopy) _city _returnvalue_3)))
      (for _array_element_2 _returnvalue_4
        (if (not (Utilities|Array|ContainsItem (Variables|Default|GetCity) _array_element_2))
          (if (not (Utilities|Array|ContainsItem _potentialcity_2 _array_element_2))
            (Utilities|Array|Add _potentialcity_2 _array_element_2))))
      (Utilities|FlowControl|Delay 0.5)
      (CallFunction|CityGrowth))))

(event EventBeginPlay)

(fn ConstructionScript)