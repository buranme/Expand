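; BP_SphericalCamera is an orbit camera actor driven by screen-edge scrolling and the mouse wheel.
; BeginPlay locks the mouse to the viewport in Game and UI mode.
; Tick rotates the actor when the normalised cursor position reaches an edge: world-space yaw, local pitch checked against ±90°, in fixed per-frame steps.
; The wheel zooms by sliding the Cameraman component along local X, bounded by MinDistance and twice that value.
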(event EventBeginPlay
  (Input|SetInputModeGameandUI (Game|GetPlayerController 0) 0 "LockAlways" true))

(event Collision|EventActorBeginOverlap
  (params (OtherActor :type Actor%20Object%20Reference)))

(event EventTick
  (params (DeltaSeconds :type Float%20%28single-precision%29))
  (bind _returnvalue (Viewport|GetViewportSize))
  (bind _returnvalue_2 (Class|WidgetLayoutLibrary|GetViewportScale))
  (bind _returnvalue_3 (Transformation|GetActorRotation))
  (bind _returnvalue_4 (/ _returnvalue _returnvalue_2))
  (bind _returnvalue_5 (Class|WidgetLayoutLibrary|GetMousePositiononViewport))
  (Utilities|FlowControl|Sequence
    (:then_0
      (Math|Float|CompareFloat (/ (.x _returnvalue_5) (.x _returnvalue_4)) 0.0
        (:>
          _)
        (:==
          _))
      (Math|Float|CompareFloat (/ (.x _returnvalue_5) (.x _returnvalue_4)) 1.0
        (:==
          _)
        (:<
          _))
      (Math|Float|CompareFloat (/ (.x _returnvalue_5) (.x _returnvalue_4)) 0.01
        (:>
          (Math|Float|CompareFloat (/ (.x _returnvalue_5) (.x _returnvalue_4)) 0.99
            (:>
              (Class|Actor|AddActorWorldRotation "0.000000,-0.100000,0.000000"))))
        (:<
          (Class|Actor|AddActorWorldRotation "0.000000,0.100000,0.000000"))))
    (:then_1
      (Math|Float|CompareFloat (/ (.y _returnvalue_5) (.y _returnvalue_4)) 0.0
        (:>
          _)
        (:==
          _))
      (Math|Float|CompareFloat (/ (.y _returnvalue_5) (.y _returnvalue_4)) 1.0
        (:==
          _)
        (:<
          _))
      (Math|Float|CompareFloat (/ (.y _returnvalue_5) (.y _returnvalue_4)) 0.01
        (:>
          (Math|Float|CompareFloat (/ (.y _returnvalue_5) (.y _returnvalue_4)) 0.99
            (:>
              (Math|Float|CompareFloat (.pitch _returnvalue_3) 9e+01
                (:<
                  (Transformation|AddActorLocalRotation "0.250000, 0, 0" false false))))))
        (:<
          (Math|Float|CompareFloat (.pitch _returnvalue_3) -9e+01
            (:>
              (Transformation|AddActorLocalRotation "-0.250000, 0, 0" false false))))))))

(event Input|MouseEvents|MouseWheelUp
  (params (Key :type Key%20Structure :default "None"))
  (bind _cameraman (Variables|Default|GetCameraman))
  (:Pressed
    (Math|Float|CompareFloat (.x (Variables|/Script/Engine.SceneComponent|GetRelativeLocation _cameraman)) (Variables|Default|GetMinDistance)
      (:==
        _)
      (:<
        _))
    (Transformation|AddRelativeLocation _cameraman "10.000000, 0, 0" false false)))

(event Input|MouseEvents|MouseWheelDown
  (params (Key :type Key%20Structure :default "None"))
  (bind _cameraman (Variables|Default|GetCameraman))
  (:Pressed
    (Math|Float|CompareFloat (.x (Variables|/Script/Engine.SceneComponent|GetRelativeLocation _cameraman)) (* (Variables|Default|GetMinDistance) 2.0)
      (:>
        _)
      (:==
        _))
    (Transformation|AddRelativeLocation _cameraman "-10.000000, 0, 0" false false)))

(fn ConstructionScript)