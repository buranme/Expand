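; Planet actor that gives its spherical mesh a dynamic planet material with a random noise offset and a sea level set from its radius.
; In Game_Level it calls CreateSphere, fits the spherical camera to the radius and animates average temperature through a timeline.
; Elsewhere it only looks up the menu camera.
; Keys save or clear planet data via the game instance and toggle a pausing escape menu.
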(event EventBeginPlay
  (bind _radius (Variables|Default|GetRadius))
  (bind _returnvalue (* _radius -1.2))
  (Input|EnableInput (Game|GetPlayerController 0))
  (bind _asbp_game_instance (Utilities|Casting|CastToBP_Game_Instance (Game|GetGameInstance)))
  (Variables|Default|SetGameInstanceRef _asbp_game_instance)
  (bind _returnvalue_2 (Rendering|Material|CreateDynamicMaterialInstance "/Game/Materials/M_Planet_Material.M_Planet_Material" "None" "None" :!class /Script/Engine.KismetMaterialLibrary))
  (bind _output_get (Variables|Default|SetCreatedMI _returnvalue_2))
  (Rendering|Material|SetVectorParameterValue _output_get "NoiseRandom" (Math|Conversions|ToLinearColor(Vector) (* (Math|Random|RandomUnitVector) 1e+03)) :!class /Script/Engine.MaterialInstanceDynamic)
  (Rendering|Material|SetScalarParameterValue _output_get "SeaLevel" (Variables|Default|GetRadius) :!class /Script/Engine.MaterialInstanceDynamic)
  (Variables|Default|SetMaterial _output_get)
  (bind _returnvalue_3 (Game|GetCurrentLevelName true))
  (if (Utilities|Enum|Equal(Enum) _returnvalue_3 "Game_Level")
    (Class|SphericalMesh|CreateSphere)
    (bind _returnvalue_4 (Actor|GetActorOfClass "/Game/Blueprints/BP_SphericalCamera.BP_SphericalCamera_C"))
    (Variables|/Game/Blueprints/BP_SphericalCamera.BP_SphericalCamera_C|SetMinDistance _returnvalue_4 _returnvalue)
    (Transformation|SetWorldLocation (Variables|/Script/Engine.Actor|GetRootComponent _returnvalue_4) "0, 0, 0" false false)
    (Transformation|SetRelativeLocation (Variables|/Game/Blueprints/BP_SphericalCamera.BP_SphericalCamera_C|GetCameraman _returnvalue_4) (Math|Vector|MakeVector _returnvalue 0.0 0.0) false false)
    (bind _curvetrack (Timeline|Timeline_0 Play)
      (:Update
        (Rendering|Material|SetScalarParameterValue (Variables|Default|GetCreatedMI) "AverageTemperature" _curvetrack :!class /Script/Engine.MaterialInstanceDynamic)))
    (else
      (bind _returnvalue_5 (Actor|GetActorOfClass "/Game/Blueprints/BP_Main_Menu_Camera.BP_Main_Menu_Camera_C")))))

(event Input|KeyboardEvents|S
  (params (Key :type Key%20Structure :default "None"))
  (bind _gameinstanceref (Variables|Default|GetGameInstanceRef))
  (:Pressed
    (Variables|/Game/Blueprints/BP_Game_Instance.BP_Game_Instance_C|SetPlanet _gameinstanceref self)
    (Default|SavePlanetData _gameinstanceref)))

(event Input|KeyboardEvents|Escape
  (params (Key :type Key%20Structure :default "None"))
  (:Pressed
    (if (Game|IsGamePaused)
      (Widget|RemovefromParent (Variables|Default|GetEscapeMenu))
      (Game|SetGamePaused false)
      (else
        (bind _returnvalue (UserInterface|CreateWidget "/Game/Widgets/W_Escape_Menu.W_Escape_Menu_C"))
        (bind _output_get (Variables|Default|SetEscapeMenu _returnvalue))
        (UserInterface|Viewport|AddtoViewport _returnvalue 0)
        (Game|SetGamePaused true)))))

(event Input|KeyboardEvents|SpaceBar
  (params (Key :type Key%20Structure :default "None"))
  (:Pressed
    (Default|ClearPlanetData (Variables|Default|GetGameInstanceRef))))

(fn ConstructionScript)